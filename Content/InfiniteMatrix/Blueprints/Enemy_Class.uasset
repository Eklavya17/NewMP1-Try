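; Enemy actor for InfiniteMatrix that dies when shot and damages the player on contact.
; All logic runs from the Box component's hit event, which casts the other actor to Projectile or BP_Player.
; A projectile hit destroys the enemy, while a player hit subtracts clamped health and also destroys it.
; When that leaves health at zero, it flags the player dead and calls the player's restart display.
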(event `self.Box.OnComponentHit`
  (params (HitComponent :type "PrimitiveComponent Object Reference") (OtherActor :type "Actor Object Reference") (OtherComp :type "PrimitiveComponent Object Reference") (NormalImpulse :type "Vector Structure") (Hit :type "HitResult Structure (by ref)"))
  (cast `/Game/InfiniteMatrix/Blueprints/Projectile` OtherActor
    (:`then`
      (`self.K2_DestroyActor`))
    (:`CastFailed`
      (bind _asbp_player (cast `/Game/InfiniteMatrix/Blueprints/BP_Player` OtherActor))
      (bind _output_get (set `/Game/InfiniteMatrix/Blueprints/BP_Player.Health` (`KismetMathLibrary.FClamp` (- (`/Game/InfiniteMatrix/Blueprints/BP_Player.Health` _asbp_player) 30.0) 0.0 100.0) _asbp_player))
      (`self.K2_DestroyActor`)
      (`/Engine/EditorBlueprintResources/StandardMacros.CompareFloat` _output_get
        (:`==`
          (set `/Game/InfiniteMatrix/Blueprints/BP_Player.IsDead` true _asbp_player)
          (`/Game/InfiniteMatrix/Blueprints/BP_Player.DisplayRestart` _asbp_player))))))

(fn `UserConstructionScript`)